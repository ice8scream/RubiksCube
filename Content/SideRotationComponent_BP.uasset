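; Actor component on MyCube that turns one side of a Rubik's-style 3x3x3 cube by mouse drag.
; Bound cube events attach the side to a rotation center and pick its axis, while Tick converts horizontal or vertical drag into an angle.
; On release, Tick rotates to the nearest quarter turn, then rounds the rotation, reattaches pieces to the cube and recalculates their Parts indices from position.
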(event Custom|StartRotation
  (params (RotationAxisIndex :type Integer) (RotationRowIndex :type Integer) (IsInputHorisontal :type Boolean) (ClickPosition :type Vector%202D%20Structure))
  (Variables|Default|SetRotationAxisIndex RotationAxisIndex)
  (Variables|Default|SetRotationRowIndex RotationRowIndex)
  (Variables|Default|SetIsInputHorisontal IsInputHorisontal)
  (Variables|Default|SetClickPosition ClickPosition)
  (if (not (Variables|Default|GetIsSideAttached))
    (Class|Cube|AttachSidetoRotatationCenter (Variables|Default|GetCube) (Variables|Default|GetRotationAxisIndex) (Variables|Default|GetRotationRowIndex))
    (switch int (Variables|Default|GetRotationAxisIndex)
      (:0
        (Variables|Default|SetSideRotation "0, 0,-1.000000"))
      (:1
        (Variables|Default|SetSideRotation "1.000000, 0, 0"))
      (:2
        (Variables|Default|SetSideRotation "0,-1.000000, 0")))
    (Variables|Default|SetIsSideAttached true)
    (Variables|Default|SetIs%20InputPressed true)))

(event Custom|EndRotation
  (bind _rotationangle (Variables|Default|GetRotationAngle))
  (bind _returnvalue (/ _rotationangle 9e+01))
  (if (Variables|Default|GetIs%20InputPressed)
    (Variables|Default|SetIs%20InputPressed false)
    (if (> (- (Math|Conversions|ToFloat(Integer) (Math|Float|Round _returnvalue)) _returnvalue) 0.0)
      (Variables|Default|SetRotationToFixDirection 1.0)
      (else
        (Variables|Default|SetRotationToFixDirection -1.0)))))

(event EventBeginPlay
  (bind _asmy_cube (Utilities|Casting|CastToMyCube (Components|GetOwner)))
  (bind _output_get (Variables|Default|SetCube _asmy_cube))
  (Variables|Default|SetRotationCenter (Variables|/Script/RubiksCube.Cube|GetRotationCenter _output_get))
  (EventDispatchers|BindEventtoSideStartRotation (Variables|Default|GetCube) (delegate Custom|StartRotation))
  (EventDispatchers|BindEventtoSideEndRotation (Variables|Default|GetCube) (delegate Custom|EndRotation)))

(event EventTick
  (params (DeltaSeconds :type Float%20%28single-precision%29))
  (bind _returnvalue (Game|GetPlayerController 0))
  (bind _rotationtofixdirection (Variables|Default|GetRotationToFixDirection))
  (bind _clickposition (Variables|Default|GetClickPosition))
  (bind _rotationspeed (Variables|Default|GetRotationSpeed))
  (bind (_locationx _locationy) (Game|Player|GetMousePosition _returnvalue))
  (bind _returnvalue_2 (Math|Vector2D|MakeVector2D _locationx _locationy))
  (bind _returnvalue_3 (- _returnvalue_2 _clickposition))
  (if (Variables|Default|GetIsSideAttached)
    (if (Variables|Default|GetIs%20InputPressed)
      (if (Variables|Default|GetIsInputHorisontal)
        (Variables|Default|SetRotationAngle (* (.x _returnvalue_3) _rotationspeed))
        (else
          (Variables|Default|SetRotationAngle (* (.y _returnvalue_3) _rotationspeed))))
      (Transformation|SetWorldRotation (Variables|Default|GetRotationCenter) (* (Variables|Default|GetSideRotation) (Variables|Default|GetRotationAngle)) false false)
      (elif (< (* (Math|Float|%(Float) (+ (Math|Float|%(Float) (+ (Variables|Default|GetRotationAngle) (* (Variables|Default|GetRotationToFixDirection) DeltaSeconds (Variables|Default|GetRotationToFixSpeed))) 9e+01) 9e+01) 9e+01) _rotationtofixdirection) (* (Math|Float|%(Float) (+ (Math|Float|%(Float) (Variables|Default|GetRotationAngle) 9e+01) 9e+01) 9e+01) _rotationtofixdirection))
        (Variables|Default|SetIsSideAttached false)
        (CallFunction|FixRotation)
        (CallFunction|DetachfromRotationCenter)
        (else
          (Variables|Default|SetRotationAngle (+ (Variables|Default|GetRotationAngle) (* (Variables|Default|GetRotationToFixDirection) DeltaSeconds (Variables|Default|GetRotationToFixSpeed))))
          (Transformation|SetWorldRotation (Variables|Default|GetRotationCenter) (* (Variables|Default|GetSideRotation) (Variables|Default|GetRotationAngle)) false false))))))

(fn DetachfromRotationCenter
  (LocalVariables|SetPartsToDetach (Components|GetChildrenComponents (Variables|Default|GetRotationCenter) false))
  (for _array_element (LocalVariables|GetPartsToDetach)
    (Transformation|AttachComponentToComponent _array_element (Variables|/Script/Engine.Actor|GetRootComponent (Variables|Default|GetCube)) "None" "KeepWorld" "KeepWorld" "KeepRelative" false)
    (CallFunction|SetPartNewIndex (- (Transformation|GetWorldLocation _array_element) (Transformation|GetActorLocation (Variables|Default|GetCube))) _array_element))
  (Transformation|SetWorldRotation (Variables|Default|GetRotationCenter) "0, 0, 0" false false))

(fn SetPartNewIndex
  (params (PartNewLocation :type Vector) (PartReference :type Scene%20Component%20Object%20Reference))
  (bind _returnvalue (+ PartNewLocation "100.000000,100.000000,100.000000"))
  (bind _returnvalue_2 (/ _returnvalue 100))
  (bind (_x _y _z) (Math|Vector|BreakVector _returnvalue_2))
  (bind _asstatic_mesh_component (Utilities|Casting|CastToStaticMeshComponent PartReference))
  (Utilities|Array|SetArrayElem (Variables|/Script/RubiksCube.Cube|GetParts (Variables|Default|GetCube)) (+ (Math|Float|Round _x) (* (Math|Float|Round _y) 3) (* (- 2 (Math|Float|Round _z)) 9)) _asstatic_mesh_component))

(fn FixRotation
  (bind _rotationcenter (Variables|Default|GetRotationCenter))
  (bind _returnvalue (Transformation|GetWorldRotation _rotationcenter))
  (Transformation|SetWorldRotation _rotationcenter (Math|Rotator|MakeRotator (* (Math|Float|Round (/ (.roll _returnvalue) 9e+01)) 9e+01) (* (Math|Float|Round (/ (.pitch _returnvalue) 9e+01)) 9e+01) (* (Math|Float|Round (/ (.yaw _returnvalue) 9e+01)) 9e+01)) false false))