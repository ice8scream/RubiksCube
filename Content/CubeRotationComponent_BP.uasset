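; Actor component that lets the player rotate a whole MyCube, a 3x3x3 puzzle cube, by dragging the mouse.
; Cube start and end events drive it, choosing the axis from drag orientation and, for vertical drags, screen half.
; Tick follows the mouse while pressed, then on release spins to the nearest 90-degree step.
; Once snapped, it re-indexes the cube's Parts by world position and resets RotationCenter.
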(event Custom|StartRotation
  (params (IsInputHorisontal :type Boolean) (ClickPosition :type Vector%202D%20Structure))
  (Variables|Default|SetIsInputPressed true)
  (Variables|Default|SetIsInputHorisontal IsInputHorisontal)
  (Variables|Default|SetStartClickPosition ClickPosition)
  (if (not (Variables|Default|GetIsCubeRotationInitialise))
    (Variables|Default|SetIsCubeRotationInitialise true)
    (if IsInputHorisontal
      (Variables|Default|SetRotation "0.000000,1.000000,0.000000")
      (elif (> (.x (Variables|Default|GetStartClickPosition)) (/ (.x (Viewport|GetViewportSize)) 2.0))
        (Variables|Default|SetRotation "-1.000000,0.000000,0.000000")
        (else
          (Variables|Default|SetRotation "0.000000,0.000000,1.000000"))))
    (Variables|Default|SetCubeStartRotation (Transformation|GetActorRotation (Variables|Default|GetCube)))
    (Variables|Default|SetIsCubeSpinning true)))

(event Custom|EndRotation
  (bind _rotationangle (Variables|Default|GetRotationAngle))
  (bind _returnvalue (/ _rotationangle 9e+01))
  (if (> (- (Math|Conversions|ToFloat(Integer) (Math|Float|Round _returnvalue)) _returnvalue) 0.0)
    (Variables|Default|SetRotationToFixDirection 1.0)
    (else
      (Variables|Default|SetRotationToFixDirection -1.0)))
  (Variables|Default|SetIsInputPressed false))

(event EventBeginPlay
  (bind _asmy_cube (Utilities|Casting|CastToMyCube (Components|GetOwner)))
  (bind _output_get (Variables|Default|SetCube _asmy_cube))
  (EventDispatchers|BindEventtoCubeStartRotation _output_get (delegate Custom|StartRotation))
  (EventDispatchers|BindEventtoCubeEndRotation _output_get (delegate Custom|EndRotation)))

(event EventTick
  (params (DeltaSeconds :type Float%20%28single-precision%29))
  (bind _returnvalue (Game|GetPlayerController 0))
  (bind _rotationtofixdirection (Variables|Default|GetRotationToFixDirection))
  (bind _cube (Variables|Default|GetCube))
  (bind _startclickposition (Variables|Default|GetStartClickPosition))
  (bind _returnvalue_2 (Transformation|GetActorRotation _cube))
  (bind (_locationx _locationy) (Game|Player|GetMousePosition _returnvalue))
  (if (Variables|Default|GetIsCubeSpinning)
    (if (Variables|Default|GetIsInputPressed)
      (if (Variables|Default|GetIsInputHorisontal)
        (Variables|Default|SetRotationAngle (* (- (.x _startclickposition) _locationx) (Variables|Default|GetRotationSpeed)))
        (else
          (Variables|Default|SetRotationAngle (* (Variables|Default|GetRotationSpeed) (- (.y _startclickposition) _locationy)))))
      (Transformation|SetActorRotation (Variables|Default|GetCube) (Math|Rotator|CombineRotators (Variables|Default|GetCubeStartRotation) (* (Variables|Default|GetRotation) (Variables|Default|GetRotationAngle))))
      (elif (< (* (Math|Float|%(Float) (+ (Math|Float|%(Float) (+ (Variables|Default|GetRotationAngle) (* (Variables|Default|GetRotationToFixDirection) (Utilities|Time|GetWorldDeltaSeconds) (Variables|Default|GetRotationToFixSpeed))) 9e+01) 9e+01) 9e+01) _rotationtofixdirection) (* (Math|Float|%(Float) (+ (Math|Float|%(Float) (Variables|Default|GetRotationAngle) 9e+01) 9e+01) 9e+01) _rotationtofixdirection))
        (Variables|Default|SetIsCubeSpinning false)
        (Transformation|SetActorRotation _cube (Math|Rotator|MakeRotator (* (Math|Float|Round (/ (.roll _returnvalue_2) 9e+01)) 9e+01) (* (Math|Float|Round (/ (.pitch _returnvalue_2) 9e+01)) 9e+01) (* (Math|Float|Round (/ (.yaw _returnvalue_2) 9e+01)) 9e+01)))
        (Variables|Default|SetPartsToReCount (Variables|/Script/RubiksCube.Cube|GetParts (Variables|Default|GetCube)))
        (for _array_element (Variables|Default|GetPartsToReCount)
          (Utilities|Array|SetArrayElem (Variables|/Script/RubiksCube.Cube|GetParts (Variables|Default|GetCube)) (+ (Math|Float|Round (.X (Math|Vector|BreakVector (/ (+ (- (Transformation|GetWorldLocation _array_element) (Transformation|GetActorLocation (Variables|Default|GetCube))) "100.000000,100.000000,100.000000") 100)))) (* (Math|Float|Round (.Y (Math|Vector|BreakVector (/ (+ (- (Transformation|GetWorldLocation _array_element) (Transformation|GetActorLocation (Variables|Default|GetCube))) "100.000000,100.000000,100.000000") 100)))) 3) (* (- 2 (Math|Float|Round (.Z (Math|Vector|BreakVector (/ (+ (- (Transformation|GetWorldLocation _array_element) (Transformation|GetActorLocation (Variables|Default|GetCube))) "100.000000,100.000000,100.000000") 100))))) 9)) _array_element))
        (Transformation|SetWorldRotation (Variables|/Script/RubiksCube.Cube|GetRotationCenter (Variables|Default|GetCube)) "0, 0, 0" false false)
        (Variables|Default|SetIsCubeRotationInitialise false)
        (else
          (Variables|Default|SetRotationAngle (+ (Variables|Default|GetRotationAngle) (* (Variables|Default|GetRotationToFixDirection) (Utilities|Time|GetWorldDeltaSeconds) (Variables|Default|GetRotationToFixSpeed))))
          (Transformation|SetActorRotation (Variables|Default|GetCube) (Math|Rotator|CombineRotators (Variables|Default|GetCubeStartRotation) (* (Variables|Default|GetRotation) (Variables|Default|GetRotationAngle)))))))))

(fn StopRotation)